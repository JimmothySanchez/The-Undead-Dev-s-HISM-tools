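; Scatter actor that fills a HierarchicalInstancedStaticMesh with randomized mesh instances around itself from the construction script.
; Each instance takes the XY of a random unit vector scaled by ScatterRadius, offset from the root.
; An optional line trace along ScatterStampDirection stamps it onto surfaces, then a height offset applies.
; Rotation is random, optionally yaw-only, and uniform scale varies by ScaleVariance.
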(fn `UserConstructionScript`
  (locals (lclMeshLocation :type "Vector Structure" :default (0.0 0.0 0.0)) (lclMeshRot :type "Rotator Structure" :default (struct)) (lclScale :type "Float (double-precision)" :default 0.0) (lclMeshIndex :type Integer))
  (for _index (range (`self.MeshCount`))
    (set `local.lclMeshIndex` _index)
    (`|ExecutionSequence`
      (:`then_0`
        ;[1 1 1] Get Location on Circle
        (set `local.lclMeshLocation` (+ (`KismetMathLibrary.MakeVector` (.x (* (`KismetMathLibrary.RandomUnitVector`) (`self.ScatterRadius`))) (.y (* (`KismetMathLibrary.RandomUnitVector`) (`self.ScatterRadius`)))) (`SceneComponent.K2_GetComponentLocation` (`self.DefaultSceneRoot`)))))
      (:`then_1`
        ;[1 1 1] Stamp
        (if (`self.StampToSurface`)
          (bind (_outhit _returnvalue) (`KismetSystemLibrary.LineTraceSingle` (`local.lclMeshLocation`) (+ (`local.lclMeshLocation`) (* (`self.ScatterStampDirection`) 100000.0)) "TraceTypeQuery1" false (`|MakeArray` null :!type "Actor Object Reference") "None" true (struct :`R` 1.0 :`A` 1.0) (struct :`R` 1.0 :`B` 0.595898 :`A` 1.0)))
          (if _returnvalue
            (set `local.lclMeshLocation` (`.Location` (`GameplayStatics.BreakHitResult` _outhit))))))
      (:`then_2`
        ;[1 1 1] Height offset
        (if (!= (`self.HeightOffset`) 0.0)
          (set `local.lclMeshLocation` (`KismetMathLibrary.MakeVector` (.x (`local.lclMeshLocation`)) (.y (`local.lclMeshLocation`)) (+ (.z (`local.lclMeshLocation`)) (`self.HeightOffset`))))))
      (:`then_3`
        ;[1 1 1] Define Rot
        (if (`self.LockVerticalRotation`)
          (set `local.lclMeshRot` (`KismetMathLibrary.MakeRotator` 0.0 0.0 (`KismetMathLibrary.RandomFloatInRange` 0.0 360.0)))
          (else
            (set `local.lclMeshRot` (`KismetMathLibrary.MakeRotator` (`KismetMathLibrary.RandomFloatInRange` 0.0 360.0) (`KismetMathLibrary.RandomFloatInRange` 0.0 360.0) (`KismetMathLibrary.RandomFloatInRange` 0.0 360.0))))))
      (:`then_4`
        ;[1 1 1] Set Scale
        (set `local.lclScale` (`KismetMathLibrary.RandomFloatInRange` (`KismetMathLibrary.FClamp` (- 1.0 (`self.ScaleVariance`)) 0.0 1000.0) (+ (`self.ScaleVariance`) 1.0))))
      (:`then_5`
        ;[1 1 1] Spawn
        (`InstancedStaticMeshComponent.AddInstanceWorldSpace` (`self.HierarchicalInstancedStaticMesh`) (`KismetMathLibrary.MakeTransform` (`local.lclMeshLocation`) (`local.lclMeshRot`) (* (`KismetMathLibrary.MakeVector` 1.0 1.0 1.0) (`local.lclScale`))))))))